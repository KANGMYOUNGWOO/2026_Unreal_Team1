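; BP_Skill_Charge_Laser is a ball skill that charges briefly, then fires a laser effect.
; Preparing starts a drain Niagara effect and activates the skill after a short delay.
; Activation starts the laser Niagara system, whose finish callback completes the skill, while stopping or finishing deactivates it.
; Hits spawn an enlarged, auto-released slash burst at the hit location.
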(event `self.PrepareSkill`
  ; Prepare
  (`ActorComponent.SetActive` (`self.Drain Niagara`) true true)
  (`KismetSystemLibrary.Delay` 0.75)
  (`self.ActivateSkill`))

(event `self.OnHit`
  (params (Target :type "Actor Object Reference") (AppliedDamage :type Integer) (HitLocation :type "Vector Structure"))
  ; On Hit
  (bind _returnvalue (`NiagaraFunctionLibrary.SpawnSystemAtLocation` "/Game/UnityParticle/Burst_Slash.Burst_Slash" HitLocation (struct) (1.0 1.0 1.0) true true "AutoRelease"))
  (`FXSystemComponent.SetFloatParameter` _returnvalue "EmitterScale" 12.0))

(event `self.OnActivated`
  (bind _laser_niagara (`self.Laser Niagara`))
  (`ActorComponent.SetActive` _laser_niagara true true)
  (add `NiagaraComponent.OnSystemFinished` _laser_niagara (delegate `Niagara Finished`)))

(event `Niagara Finished`
  (params (PSystem :type "NiagaraComponent Object Reference"))
  (`self.CompleteSkill`))

(event `self.OnStopped`
  (`ActorComponent.Deactivate` (`self.Laser Niagara`) :!label _label))

(event `self.OnFinished`
  (goto _label))

(fn `UserConstructionScript`)