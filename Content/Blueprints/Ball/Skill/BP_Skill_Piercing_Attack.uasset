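; BP_Skill_Piercing_Attack is a ball skill that handles the presentation and lifetime of a piercing attack.
; Activation restarts the attack Niagara effect and plays a spin sound, and the skill completes when that effect's system finishes.
; Each hit spawns an auto-released, scaled-up slash burst at the hit location and triggers hit feedback through SkillFeedbackComponent.
; Stopping or finishing the skill deactivates the attack effect.
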(event `self.OnHit`
  (params (Target :type "Actor Object Reference") (AppliedDamage :type Integer) (HitLocation :type "Vector Structure"))
  ; Comment
  (bind _returnvalue (`NiagaraFunctionLibrary.SpawnSystemAtLocation` "/Game/UnityParticle/Burst_Slash.Burst_Slash" HitLocation (struct) (1.0 1.0 1.0) true true "AutoRelease"))
  (`FXSystemComponent.SetFloatParameter` _returnvalue "EmitterScale" 12.0)
  (`PBSkillFeedbackComponent.PlayHitFeedback` (`self.SkillFeedbackComponent`)))

(event `self.OnActivated`
  (`ActorComponent.SetActive` (`self.Attack Niagara`) true true)
  (add `NiagaraComponent.OnSystemFinished` (`self.Attack Niagara`) (delegate `OnSystemFinished_Event`))
  (`PBSkillFeedbackComponent.PlaySkillSound` (`self.SkillFeedbackComponent`) "/Game/Resources/Sound/SFX/S_Spin.S_Spin" 1.0 1.0))

(event `self.OnStopped`
  (`ActorComponent.Deactivate` (`self.Attack Niagara`) :!label _label))

(event `OnSystemFinished_Event`
  (params (PSystem :type "NiagaraComponent Object Reference"))
  (`self.CompleteSkill`))

(event `self.OnFinished`
  (goto _label))

(fn `UserConstructionScript`)