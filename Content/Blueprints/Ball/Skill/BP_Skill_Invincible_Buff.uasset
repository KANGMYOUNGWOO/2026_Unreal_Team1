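; Ball skill Blueprint for the Invincible buff, handling its aura visuals and completion timing.
; Activation restarts the NiagaraOra effect and plays AppearSequence forward.
; The skill completes when the Niagara system finishes, so the effect's length drives that completion.
; Stopping or finishing deactivates the aura and plays the sequence in reverse; no invincibility logic appears in this graph.
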(event `self.OnActivated`
  (`ActorComponent.SetActive` (`self.Niagara_Ora`) true true)
  (`ActorSequenceComponent.PlaySequence` (`self.Appear Sequence`))
  (add `NiagaraComponent.OnSystemFinished` (`self.Niagara_Ora`) (delegate `OnSystemFinished_Event`)))

(event `OnSystemFinished_Event`
  (params (PSystem :type "NiagaraComponent Object Reference"))
  (`self.CompleteSkill`))

(event `self.OnStopped`
  (`ActorComponent.Deactivate` (`self.Niagara_Ora`) :!label _label)
  (`ActorSequenceComponent.PlaySequenceReverse` (`self.Appear Sequence`)))

(event `self.OnFinished`
  (goto _label))

(fn `UserConstructionScript`)