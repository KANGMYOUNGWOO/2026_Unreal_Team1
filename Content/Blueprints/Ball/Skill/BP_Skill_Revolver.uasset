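; Revolver skill Blueprint for a ball, providing the visual and audio reaction when the gun fires.
; OnFired triggers the muzzle burst and plays a pitch-randomized gunshot through SkillFeedbackComponent.
; It also snaps the root to the fire direction and zeroes RotatingMovement, holding the aim briefly before setting a fast spin again.
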(event `self.OnFired`
  (params (FireDirection :type "Vector Structure"))
  (bind _rotatingmovement (`self.RotatingMovement`))
  (`|ExecutionSequence`
    (:`then_0`
      (`ActorComponent.Activate` (`self.Burst_Muzzle`) true)
      (`PBSkillFeedbackComponent.PlaySkillSound` (`self.SkillFeedbackComponent`) "/Game/Resources/Sound/SFX/Battle/S_GunShot.S_GunShot" 1.0 (`KismetMathLibrary.RandomFloatInRange` 0.9 1.1)))
    (:`then_1`
      (`SceneComponent.K2_SetRelativeRotation` (`self.Root`) (`KismetMathLibrary.MakeRotFromX` FireDirection) false false)
      (set `RotatingMovementComponent.RotationRate` (struct) _rotatingmovement)
      (`KismetSystemLibrary.Delay` 1.0)
      (set `RotatingMovementComponent.RotationRate` (struct :`Yaw` 1600.0) _rotatingmovement))))

(fn `UserConstructionScript`)