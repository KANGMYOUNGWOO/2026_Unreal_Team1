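; BP_Skill_Slash is a ball skill that performs a timed slash attack when activated.
; It charges while an appear sequence plays, then starts an attack sequence after a delay.
; A sequencer event starts the attack, Niagara trail and smash sound.
; After another delay the attack ends, the trail deactivates, and the appear sequence plays in reverse before the skill completes.
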(event `self.OnActivated`
  (`self.Charge`))

(event `Charge`
  (`ActorSequenceComponent.PlaySequence` (`self.ApppearSequence`))
  (`self.StartCharge`)
  (`KismetSystemLibrary.Delay` (`self.AppearDelay`))
  (`ActorSequenceComponent.PlaySequence` (`self.AttackSequence`)))

(event `Attack`
  (`self.StartAttack`)
  (`KismetSystemLibrary.Delay` (`self.AttackDelay`))
  (`self.FinishAttack`)
  (`ActorComponent.Deactivate` (`self.Niagara Trail`)))

(event `FinishAttack`
  (`self.EndAttack`)
  (`ActorSequenceComponent.PlaySequenceReverse` (`self.ApppearSequence`))
  (`KismetSystemLibrary.Delay` (`self.AppearDelay`))
  (`self.CompleteSkill`))

(event `SequenceEvent`
  (bind _niagara_trail (`self.Niagara Trail`))
  (`self.Attack`)
  (`/Engine/EditorBlueprintResources/StandardMacros.IsValid` _niagara_trail
    (:`Is Valid`
      (`ActorComponent.Activate` _niagara_trail false)
      (`PBSkillFeedbackComponent.PlaySkillSound` (`self.SkillFeedbackComponent`) "/Game/Resources/Sound/SFX/S_Smash.S_Smash" 1.0 1.0))))

(fn `UserConstructionScript`)