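; BP_Bomb is a summoned skill bomb in the ball skill set that glows before exploding.
; BeginPlay creates a dynamic material instance on the Bomb component so the emissive level can be animated.
; RequestExplode plays a timeline that drives Emissive, then calls Explode, which is defined outside these graphs, and ShowExplode.
; ShowExplode spawns a pooled, auto-released, scaled-up burst effect at the bomb's location.
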(event `self.ReceiveBeginPlay`
  (bind _bomb (`self.Bomb`))
  (bind _returnvalue (`PrimitiveComponent.CreateDynamicMaterialInstance` _bomb 0 (`PrimitiveComponent.GetMaterial` _bomb 1) "None"))
  (set `self.Material` _returnvalue))

(event `self.RequestExplode`
  (bind (_direction _emissive) (`Timeline|Timeline` :!via `PlayFromStart`)
    (:`Update`
      (`MaterialInstanceDynamic.SetScalarParameterValue` (`self.Material`) "Emissive" _emissive))
    (:`Finished`
      (`self.Explode`)
      (`self.Show Explode`))))

(event `Show Explode`
  (bind _returnvalue (`NiagaraFunctionLibrary.SpawnSystemAtLocation` "/Game/UnityParticle/Burst_Explode.Burst_Explode" (`self.K2_GetActorLocation`) (struct) (1.0 1.0 1.0) true true "AutoRelease"))
  (`/Engine/EditorBlueprintResources/StandardMacros.IsValid` _returnvalue
    (:`Is Valid`
      (`FXSystemComponent.SetFloatParameter` _returnvalue "EmitterScale" 13.0))))

(fn `UserConstructionScript`)