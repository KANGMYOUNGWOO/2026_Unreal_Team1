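; Sword Storm ball skill Blueprint that performs a three-hit dash attack combo with a trailing effect and sharp burst on hit.
; On activation a timeline's Attack event fires DashAttack, which steps by AttackCount through two alternating attack sequences with smash sounds, re-charging between hits and ending the attack after the third.
; An appear sequence plays on spawn and reverses when the timeline finishes and completes the skill; stopping also completes it.
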(event `self.OnHit`
  (params (Target :type "Actor Object Reference") (AppliedDamage :type Integer) (HitLocation :type "Vector Structure"))
  (bind _returnvalue (`NiagaraFunctionLibrary.SpawnSystemAtLocation` "/Game/UnityParticle/Burst_Sharp.Burst_Sharp" HitLocation))
  (`/Engine/EditorBlueprintResources/StandardMacros.IsValid` _returnvalue
    (:`Is Valid`
      (`FXSystemComponent.SetFloatParameter` _returnvalue "EmitterScale" 10.0))))

(event `self.ReceiveBeginPlay`
  ; Begin play
  (`ActorSequenceComponent.PlaySequence` (`self.ApppearSequence`)))

(event `self.OnActivated`
  (bind _niagara_trail (`self.Niagara Trail`))
  (set `self.AttackCount` 0)
  (`self.StartCharge`)
  (`Timeline|Timeline` :!via `PlayFromStart` :!label _label
    (:`Finished`
      (`ActorSequenceComponent.PlaySequenceReverse` (`self.ApppearSequence`))
      (`self.CompleteSkill`))
    (:`Attack Event`
      (`self.Dash Attack`)
      (`/Engine/EditorBlueprintResources/StandardMacros.IncrementInt` (`self.AttackCount`)
        (:`  `
          (`/Engine/EditorBlueprintResources/StandardMacros.IsValid` _niagara_trail
            (:`Is Valid`
              (`ActorComponent.Activate` _niagara_trail false))))))))

(event `self.OnStopped`
  (`|ExecutionSequence`
    (:`then_0`
      (goto _label :!via `Stop`))
    (:`then_1`
      (`self.CompleteSkill`))))

(event `self.OnFinished`
  (`self.Deactive Trail`))

(event `Dash Attack`
  (bind _attacksequence02 (`self.AttackSequence02`))
  (bind _attacksequence01 (`self.AttackSequence01`))
  (bind _attacksequence01_2 (`self.AttackSequence01`))
  (switch `int` (`self.AttackCount`)
    (:`0`
      (`self.StartAttack`)
      (`/Engine/EditorBlueprintResources/StandardMacros.IsValid` _attacksequence01_2
        (:`Is Valid`
          (`ActorSequenceComponent.PlaySequence` _attacksequence01_2)
          (`PBSkillFeedbackComponent.PlaySkillSound` (`self.SkillFeedbackComponent`) "/Game/Resources/Sound/SFX/Battle/S_Smash.S_Smash" 1.0 1.0)
          (`KismetSystemLibrary.Delay` 0.3)
          (`self.StartCharge`)
          (`self.Deactive Trail`))))
    (:`1`
      (`self.StartAttack`)
      (`/Engine/EditorBlueprintResources/StandardMacros.IsValid` _attacksequence02
        (:`Is Valid`
          (`ActorSequenceComponent.PlaySequence` _attacksequence02)
          (`PBSkillFeedbackComponent.PlaySkillSound` (`self.SkillFeedbackComponent`) "/Game/Resources/Sound/SFX/Battle/S_Smash.S_Smash" 1.0 1.5)
          (`KismetSystemLibrary.Delay` 0.2)
          (`self.StartCharge`)
          (`self.Deactive Trail`))))
    (:`2`
      (`self.StartAttack`)
      (`/Engine/EditorBlueprintResources/StandardMacros.IsValid` _attacksequence01
        (:`Is Valid`
          (`ActorSequenceComponent.PlaySequence` _attacksequence01)
          (`PBSkillFeedbackComponent.PlaySkillSound` (`self.SkillFeedbackComponent`) "/Game/Resources/Sound/SFX/Battle/S_Smash.S_Smash" 1.0 1.0)
          (`KismetSystemLibrary.Delay` 0.3)
          (`self.EndAttack`)
          (`self.Deactive Trail`))))))

(fn `Deactive Trail`
  (bind _niagara_trail (`self.Niagara Trail`))
  (`/Engine/EditorBlueprintResources/StandardMacros.IsValid` _niagara_trail
    (:`Is Valid`
      (`ActorComponent.Deactivate` _niagara_trail))))

(fn `UserConstructionScript`)