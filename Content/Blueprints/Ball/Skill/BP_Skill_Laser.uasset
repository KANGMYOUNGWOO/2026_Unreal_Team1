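; BP_Skill_Laser is a ball skill Blueprint that fires a laser effect.
; Preparing activates a drain Niagara effect, then activates the skill after a short delay.
; Activation plays the laser Niagara system and completes the skill when that system finishes.
; Stopping or finishing the skill deactivates the laser effect.
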(event `self.PrepareSkill`
  (`ActorComponent.SetActive` (`self.Drain Niagara`) true true)
  (`KismetSystemLibrary.Delay` 0.75)
  (`self.ActivateSkill`))

(event `self.OnActivated`
  (bind _laser_niagara (`self.Laser Niagara`))
  (`ActorComponent.SetActive` _laser_niagara true true)
  (add `NiagaraComponent.OnSystemFinished` _laser_niagara (delegate `Niagara Finished`))
  (`KismetSystemLibrary.PrintString` "bind"))

(event `Niagara Finished`
  (params (PSystem :type "NiagaraComponent Object Reference"))
  (`self.CompleteSkill`)
  (`KismetSystemLibrary.PrintString` "complete"))

(event `self.OnStopped`
  (`ActorComponent.Deactivate` (`self.Laser Niagara`) :!label _label))

(event `self.OnFinished`
  (goto _label))

(fn `UserConstructionScript`)