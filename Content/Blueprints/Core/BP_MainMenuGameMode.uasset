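; Main menu game mode that shows the menu UI and handles the transition to the battle level.
; On BeginPlay it pushes WBP_MainMenu through the PBUIManagerSubsystem and shows the mouse cursor.
; OpenBattleLevel unloads the UI primary asset bundle via PBGameDataLoadSubsystem, opens the Lv_BumperAssetLoadTest level and hides the cursor.
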(event `self.ReceiveBeginPlay`
  ; Comment
  (`self.Add Default Widget`))

(event `Add Default Widget`
  ; Comment
  (`PBUIManagerSubsystem.PushWidget` (subsystem `PBUIManagerSubsystem`) "/Game/Blueprints/UI/MainMenu/WBP_MainMenu.WBP_MainMenu_C" 0)
  (set `PlayerController.bShowMouseCursor` true (`GameplayStatics.GetPlayerController` 0)))

(event `Open Battle Level`
  (`PBGameDataLoadSubsystem.UnloadPrimaryAssetBundleByType` (subsystem `PBGameDataLoadSubsystem`) "UI")
  (`GameplayStatics.OpenLevelBySoftObjectPtr` "/Game/Map/Test/Lv_BumperAssetLoadTest.Lv_BumperAssetLoadTest")
  (set `PlayerController.bShowMouseCursor` false (`GameplayStatics.GetPlayerController` 0)))

(fn `UserConstructionScript`)