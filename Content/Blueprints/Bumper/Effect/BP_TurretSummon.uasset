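; Bumper effect that summons a temporary turret, which scales in from zero, fires, then shrinks away.
; OnStartAction runs chained timelines for scale-in, active firing and scale-out, then calls FinishAction.
; Event keys on the active timeline trigger PBTurretFire, with a Reaction timeline offsetting the Head along its forward vector.
; HeadLookAt provides smoothed head rotation but is not called here, and LookAtTarget is unwired.
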(event `self.ReceiveBeginPlay`
  (`SceneComponent.SetRelativeScale3D` (`self.Scene`) (0.0 0.0 0.0)))

(event `self.OnStartAction`
  (params (Bumper :type "PBModularBumperBase Object Reference") (Ball :type "PBBallBase Object Reference"))
  ; 활성화 시작
  (bind (_direction _scale) (`Timeline|Timeline` :!via `PlayFromStart`)
    (:`Update`
      (`SceneComponent.SetRelativeScale3D` (`self.Scene`) (`KismetMathLibrary.Conv_DoubleToVector` _scale)))
    (:`Finished`
      (`self.Activation`))))

(event `Shoot Event`
  (bind _head (`self.Head`))
  (`|ExecutionSequence`
    (:`then_0`
      (`PBTurretFireComponent.FireOnce` (`self.PBTurretFire`)))
    (:`then_1`
      (bind (_direction _reaction) (`Timeline|Reaction` :!via `PlayFromStart`)
        (:`Update`
          (`SceneComponent.K2_SetRelativeLocation` _head (* (`SceneComponent.GetForwardVector` _head) (* _reaction 50.0)) false false))))))

(event `Activation`
  ; 포탑 활성화
  (`Timeline|Timeline_1` :!via `PlayFromStart`
    (:`Finished`
      (`self.Disappear`))
    (:`Shoot Event`
      (`self.Shoot Event`))))

(event `Disappear`
  ; 활성화 종료
  (bind (_direction _scale) (`Timeline|Timeline_0` :!via `ReverseFromEnd`)
    (:`Update`
      (`SceneComponent.SetRelativeScale3D` (`self.Scene`) (`KismetMathLibrary.Conv_DoubleToVector` _scale)))
    (:`Finished`
      (`self.FinishAction`))))

(fn `HeadLookAt`
  (params (Target1 :type "Vector Structure (by ref)") (Speed :type "Float (double-precision)" :default 10.0))
  (`SceneComponent.K2_SetWorldRotation` (`self.Head`) (`KismetMathLibrary.RLerp` (`SceneComponent.K2_GetComponentRotation` (`self.Head`)) (`KismetMathLibrary.Conv_VectorToRotator` Target1) (* Speed (`GameplayStatics.GetWorldDeltaSeconds`)) true) false false))

(fn `UserConstructionScript`)