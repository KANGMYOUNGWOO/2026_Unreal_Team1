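; BP_Side_Trigger is a bumper side trigger that displays its owning bumper's trigger progress as a gauge on its mesh.
; On BeginPlay it creates a dynamic instance of the side gauge material and, if the owner bumper is valid, binds to trigger progress changes.
; Each change sets the material's GaugeAmount parameter to the clamped ratio of current to required count, so updates are event-driven.
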(event `self.ReceiveBeginPlay`
  (bind _returnvalue (`PrimitiveComponent.CreateDynamicMaterialInstance` (`self.Mesh`) 1 "/Game/Resources/Bumper/Material/MI_BumperGauge_Side.MI_BumperGauge_Side" "None"))
  (set `self.GaugeMID` _returnvalue)
  (`/Engine/EditorBlueprintResources/StandardMacros.IsValid` (`self.GetOwnerBumper`)
    (:`Is Valid`
      (add `self.OnTriggerProgressChanged` (delegate `HandleGaugeChanged`)))))

(event `HandleGaugeChanged` :!signature `self.OnTriggerProgressChanged`
  (params (CurrentCount :type Integer) (RequiredCount :type Integer))
  (`MaterialInstanceDynamic.SetScalarParameterValue` (`self.GaugeMID`) "GaugeAmount" (`KismetMathLibrary.FClamp` (/ (`KismetMathLibrary.Conv_IntToDouble` CurrentCount) (`KismetMathLibrary.Conv_IntToDouble` RequiredCount)))))

(fn `UserConstructionScript`)