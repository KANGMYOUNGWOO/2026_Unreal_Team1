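; BP_GateBumper is a bumper trigger gate that displays its owner bumper's trigger progress as a gauge on its mesh.
; On BeginPlay it creates a dynamic gauge material on the mesh and, if the owner bumper is valid, binds to trigger progress changes.
; Each change sets the gauge amount to the clamped ratio of current to required count.
; Activation currently only prints a debug string.
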(event `self.ReceiveBeginPlay`
  (bind _returnvalue (`PrimitiveComponent.CreateDynamicMaterialInstance` (`self.Mesh`) 1 "/Game/Blueprints/Bumper/Art/Material/MI_BumperGauge_Gate.MI_BumperGauge_Gate" "None"))
  (set `self.GaugeMID` _returnvalue)
  (bind _output_get (set `self.OwnerBumperRef` (`self.GetOwnerBumper`)))
  (`/Engine/EditorBlueprintResources/StandardMacros.IsValid` _output_get
    (:`Is Valid`
      (add `self.OnTriggerProgressChanged` (delegate `HandleGaugeChanged`)))))

(event `HandleGaugeChanged` :!signature `self.OnTriggerProgressChanged`
  (params (CurrentCount :type Integer) (RequiredCount :type Integer))
  (`MaterialInstanceDynamic.SetScalarParameterValue` (`self.GaugeMID`) "GaugeAmount" (`KismetMathLibrary.FClamp` (/ (`KismetMathLibrary.Conv_IntToDouble` CurrentCount) (`KismetMathLibrary.Conv_IntToDouble` RequiredCount)))))

(event `self.OnTriggerActivated`
  (params (Ball :type "PBBallBase Object Reference") (TriggerHit :type "HitResult Structure (by ref)"))
  (`KismetSystemLibrary.PrintString` "Trigger"))

(fn `UserConstructionScript`)