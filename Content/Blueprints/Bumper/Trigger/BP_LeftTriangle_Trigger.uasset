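; BP_LeftTriangle_Trigger is a bumper trigger that displays trigger progress as a gauge on its mesh.
; On BeginPlay it creates a dynamic instance of the rebound gauge material, looks up its owner bumper and, if valid, binds to the trigger progress event.
; Each progress change writes the clamped ratio of current to required count into the material's GaugeAmount parameter.
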(event `self.ReceiveBeginPlay`
  (bind _returnvalue (`PrimitiveComponent.CreateDynamicMaterialInstance` (`self.Mesh`) 1 "/Game/Blueprints/Bumper/Art/Material/M_Rebound01Gauge.M_Rebound01Gauge" "None"))
  (set `self.GaugeMID` _returnvalue)
  (bind _output_get (set `self.OwnerBumperRef` (`self.GetOwnerBumper`)))
  (`/Engine/EditorBlueprintResources/StandardMacros.IsValid` _output_get
    (:`Is Valid`
      (add `self.OnTriggerProgressChanged` (delegate `HandleGaugeChanged`)))))

(event `HandleGaugeChanged` :!signature `self.OnTriggerProgressChanged`
  (params (CurrentCount :type Integer) (RequiredCount :type Integer))
  (`MaterialInstanceDynamic.SetScalarParameterValue` (`self.GaugeMID`) "GaugeAmount" (`KismetMathLibrary.FClamp` (/ (`KismetMathLibrary.Conv_IntToDouble` CurrentCount) (`KismetMathLibrary.Conv_IntToDouble` RequiredCount)))))

(fn `UserConstructionScript`)