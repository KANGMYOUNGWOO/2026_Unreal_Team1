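; Controller Blueprint that connects spawned modular bumpers to an on-screen bumper panel.
; On BeginPlay it binds to its OnSpawnedBumpersReady dispatcher, then creates WBP_BumperPanel for player controller 0 and adds it to the viewport.
; When the dispatcher fires, it finds all BP_ModularBumper actors in the world and binds each valid one to a panel counter by array index, ignoring the event's success flag and actor list.
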(event `self.ReceiveBeginPlay`
  (add `self.OnSpawnedBumpersReady` (delegate `Bind Widget`))
  (bind _returnvalue (`|CreateWidget` "/Game/Blueprints/Bumper/UI/WBP_BumperPanel.WBP_BumperPanel_C" (`GameplayStatics.GetPlayerController` 0)))
  (bind _output_get (set `self.Bumper Widget` _returnvalue))
  (`UserWidget.AddToViewport` _output_get 0))

(event `Bind Widget` :!signature `self.OnSpawnedBumpersReady`
  (params (bSuccess :type Boolean) (SpawnedBumperActors :type "Array of PBModularBumperBase Object Reference (by ref)"))
  (bind _outactors (`GameplayStatics.GetAllActorsOfClass` "/Game/Blueprints/Bumper/BP_ModularBumper.BP_ModularBumper_C"))
  (for (_array_element _array_index) _outactors
    (`/Engine/EditorBlueprintResources/StandardMacros.IsValid` _array_element
      (:`Is Valid`
        (`/Game/Blueprints/Bumper/UI/WBP_BumperPanel.BindToCounter` (`self.Bumper Widget`) _array_element _array_index)))))

(fn `UserConstructionScript`)